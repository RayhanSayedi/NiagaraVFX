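; BP_TextureBaker is an editor utility actor that bakes a material into a static texture asset.
; Its BakeTexture function checks that a render target and source material are set, draws the material into the target, then saves it as a Texture2D through the editor-only create call.
; It prints a status message either way, and its events and construction script are empty.
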(fn `BakeTexture`
  (bind _rendertargettodraw (`self.RenderTargetToDraw`))
  (bind _materialtodrawform (`self.MaterialToDrawForm`))
  (if (and (`KismetSystemLibrary.IsValid` _rendertargettodraw) (`KismetSystemLibrary.IsValid` _materialtodrawform))
    (`KismetSystemLibrary.PrintString` "Baking" true true (struct :`G` 1.0 :`B` 0.062942 :`A` 1.0))
    (`KismetRenderingLibrary.DrawMaterialToRenderTarget` _rendertargettodraw _materialtodrawform)
    (`KismetRenderingLibrary.RenderTargetCreateStaticTexture2DEditorOnly` (`self.RenderTargetToDraw`) "TextureFromRenderTarget")
    (else
      (`KismetSystemLibrary.PrintString` "AssetNotFound" true true (struct :`R` 1.0 :`B` 0.037431 :`A` 1.0)))))

(fn `UserConstructionScript`)